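; BP_Level is a level actor that builds a wall of bricks, apparently for a Breakout-style game.
; On BeginPlay, Generate adds static mesh components in a grid sized by Columns and Rows, roughly centered on Y and stacked upward in Z.
; A brick hit handler destroys the other component in the collision, though the file does not show where it is bound.
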(event `self.ReceiveBeginPlay`
  (`self.Generate`))

(event `Generate`
  (bind _columns (`self.Columns`))
  (for _index (range (+ _columns 1))
    (for _index_2 (range (+ (`self.Rows`) 1))
      (`AddComponent|NODE_AddStaticMeshComponent-1` :`RelativeTransform` (`KismetMathLibrary.MakeTransform` (`KismetMathLibrary.MakeVector` 0.0 (`KismetMathLibrary.Conv_IntToDouble` (* (- _index (/ _columns 2)) 150)) (`KismetMathLibrary.Conv_IntToDouble` (+ (* _index_2 90) 350))))))))

(event `OnComponentHitBrick`
  (params (HitComponent :type "PrimitiveComponent Object Reference") (OtherActor :type "Actor Object Reference") (OtherComp :type "PrimitiveComponent Object Reference") (NormalImpulse :type "Vector Structure") (Hit :type "HitResult Structure (by ref)"))
  (`ActorComponent.K2_DestroyComponent` OtherComp))

(fn `UserConstructionScript`)