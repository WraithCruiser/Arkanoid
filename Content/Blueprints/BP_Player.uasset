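; Player pawn for a brick-breaker game, combining a paddle (Cube) with a physics ball (Sphere).
; Input slides the paddle along Y with sweep, and Shoot detaches a locked ball and launches it upward with physics.
; Ball hits on bricks are forwarded to BP_Level, while hitting a Floor-tagged component destroys the ball.
; RespawnBall then creates a replacement mesh component, attaches it above the paddle and locks it for the next shot.
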(event `InputAxis|Move`
  (params (AxisValue :type "Float (single-precision)"))
  (`SceneComponent.K2_AddLocalOffset` (`self.Cube`) (`KismetMathLibrary.MakeVector` 0.0 (* AxisValue (`self.MoveSpeed`))) true false))

(event `InputAction|Shoot`
  (params (Key :type "Key Structure"))
  (bind _sphere (`self.Sphere`))
  (:`Pressed`
    (if (`self.BallLocked`)
      (`SceneComponent.K2_AttachToComponent` (`self.Sphere`) (`self.DefaultSceneRoot`) "None" "KeepWorld" "KeepWorld" "KeepWorld" true)
      (bind _output_get (set `self.BallLocked` false))
      (`PrimitiveComponent.SetSimulatePhysics` (`self.Sphere`) (not _output_get))
      (`PrimitiveComponent.SetPhysicsLinearVelocity` _sphere (`KismetMathLibrary.MakeVector` 0.0 0.0 (`self.Ball Speed`)) false "None")
      (bind _returnvalue (`PrimitiveComponent.GetPhysicsLinearVelocity` _sphere "None")))))

(event `self.ReceiveBeginPlay`
  (`SceneComponent.K2_SetWorldLocation` (`self.Sphere`) (+ (`SceneComponent.K2_GetComponentLocation` (`self.Cube`)) (0.0 0.0 25.0)) false false))

(event `self.Sphere.OnComponentHit`
  (params (HitComponent :type "PrimitiveComponent Object Reference") (OtherActor :type "Actor Object Reference") (OtherComp :type "PrimitiveComponent Object Reference") (NormalImpulse :type "Vector Structure") (Hit :type "HitResult Structure (by ref)"))
  (if (`ActorComponent.ComponentHasTag` OtherComp "Floor")
    (`self.Ball Lost`)
    (elif (and (`ActorComponent.ComponentHasTag` HitComponent "Ball") (`ActorComponent.ComponentHasTag` OtherComp "Brick"))
      (bind _asbp_level (cast `/Game/Blueprints/BP_Level` OtherActor))
      (`/Game/Blueprints/BP_Level.OnComponentHitBrick` _asbp_level HitComponent null OtherComp (0.0 0.0 0.0) Hit))))

(fn `Ball Lost`
  (`ActorComponent.K2_DestroyComponent` (`self.Sphere`))
  (`self.RespawnBall`))

(fn `RespawnBall`
  (bind _sphere (`self.Sphere`))
  (bind _cube (`self.Cube`))
  (bind _returnvalue (`AddComponent|NODE_AddStaticMeshComponent-1` :`bManualAttachment` true :`RelativeTransform` (`KismetMathLibrary.Conv_VectorToTransform` (`SceneComponent.K2_GetComponentLocation` (`self.Cube`)))))
  (`|VariableSetRef` _sphere _returnvalue)
  (`SceneComponent.SetWorldScale3D` _sphere (0.55 0.55 0.55))
  (`KismetArrayLibrary.Array_Add` (`ActorComponent.ComponentTags` _sphere) (`self.BallTag`))
  (`SceneComponent.K2_AttachToComponent` (`self.Sphere`) _cube "None" "KeepWorld" "KeepWorld" "KeepWorld" true)
  (`SceneComponent.K2_SetWorldLocation` (`self.Sphere`) (+ (`SceneComponent.K2_GetComponentLocation` _cube) (0.0 0.0 25.0)) false false)
  (set `self.BallLocked` true))

(fn `UserConstructionScript`)